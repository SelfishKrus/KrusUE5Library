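; BP_LightCam is a scene-capture actor acting as an orthographic light camera, apparently for custom shadow mapping.
; Its construction script builds a world-to-light view matrix from the capture component's location and axes, plus an orthographic projection from OrthoWidth and a hardcoded depth range.
; It writes both matrices as vector rows, plus light position, into MPC_LightParams for materials.
; Event graph logic is empty, so nothing updates on Tick.
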(event EventBeginPlay)

(event Collision|EventActorBeginOverlap
  (params (OtherActor :type Actor%20Object%20Reference)))

(event EventTick
  (params (DeltaSeconds :type Float%20%28single-precision%29)))

(fn ConstructionScript
  (bind _scenecapturecomponent2d (Variables|Default|GetSceneCaptureComponent2D))
  (bind _scenecapturecomponent2d_2 (Variables|Default|GetSceneCaptureComponent2D))
  (bind _returnvalue (Transformation|GetWorldRotation _scenecapturecomponent2d))
  (bind _returnvalue_2 (Transformation|GetWorldLocation _scenecapturecomponent2d))
  (bind _orthowidth (Variables|/Script/Engine.SceneCaptureComponent2D|GetOrthoWidth _scenecapturecomponent2d_2))
  (bind _returnvalue_3 (Math|Vector|GetForwardVector _returnvalue))
  (bind _returnvalue_4 (Math|Vector|GetRightVector _returnvalue))
  (bind _returnvalue_5 (Math|Vector|GetUpVector _returnvalue))
  (bind _returnvalue_6 (Math|Vector|DotProduct _returnvalue_3 _returnvalue_2))
  (bind _returnvalue_7 (Math|Vector|DotProduct _returnvalue_2 _returnvalue_4))
  (bind _returnvalue_8 (Math|Vector|DotProduct _returnvalue_5 _returnvalue_2))
  (bind (_x _y _z) (Math|Vector|BreakVector _returnvalue_3))
  (bind (_x_2 _y_2 _z_2) (Math|Vector|BreakVector _returnvalue_4))
  (bind (_x_3 _y_3 _z_3) (Math|Vector|BreakVector _returnvalue_5))
  (bind _returnvalue_9 (* _returnvalue_6 -1.0))
  (bind _returnvalue_10 (* _returnvalue_7 -1.0))
  (bind _returnvalue_11 (* _returnvalue_8 -1.0))
  (bind _returnvalue_12 (Math|Vector|MakeVector _returnvalue_10 _returnvalue_11 _returnvalue_9))
  (bind (_x_4 _y_4 _z_4) (Math|Vector|BreakVector _returnvalue_12))
  (Rendering|Material|SetVectorParameterValue "/Game/ShadowMap/MPC_LightParams.MPC_LightParams" "lightPos" (Math|Conversions|ToLinearColor(Vector) (Transformation|GetWorldLocation _scenecapturecomponent2d)) :!class /Script/Engine.KismetMaterialLibrary)
  (Rendering|Material|SetVectorParameterValue "/Game/ShadowMap/MPC_LightParams.MPC_LightParams" "lightMatrixX" (Utilities|Struct|MakeLinearColor _x_2 _x_3 _x 0.0) :!class /Script/Engine.KismetMaterialLibrary)
  (Rendering|Material|SetVectorParameterValue "/Game/ShadowMap/MPC_LightParams.MPC_LightParams" "lightMatrixY" (Utilities|Struct|MakeLinearColor _y_2 _y_3 _y 0.0) :!class /Script/Engine.KismetMaterialLibrary)
  (Rendering|Material|SetVectorParameterValue "/Game/ShadowMap/MPC_LightParams.MPC_LightParams" "lightMatrixZ" (Utilities|Struct|MakeLinearColor _z_2 _z_3 _z 0.0) :!class /Script/Engine.KismetMaterialLibrary)
  (Rendering|Material|SetVectorParameterValue "/Game/ShadowMap/MPC_LightParams.MPC_LightParams" "lightMatrixW" (Utilities|Struct|MakeLinearColor _x_4 _y_4 _z_4 1.0) :!class /Script/Engine.KismetMaterialLibrary)
  (Rendering|Material|SetVectorParameterValue "/Game/ShadowMap/MPC_LightParams.MPC_LightParams" "projectionX" (Utilities|Struct|MakeLinearColor (/ 2.0 _orthowidth) 0.0 0.0 0.0) :!class /Script/Engine.KismetMaterialLibrary)
  (Rendering|Material|SetVectorParameterValue "/Game/ShadowMap/MPC_LightParams.MPC_LightParams" "projectionY" (Utilities|Struct|MakeLinearColor 0.0 (/ -2.0 _orthowidth) 0.0 0.0) :!class /Script/Engine.KismetMaterialLibrary)
  (Rendering|Material|SetVectorParameterValue "/Game/ShadowMap/MPC_LightParams.MPC_LightParams" "projectionZ" (Utilities|Struct|MakeLinearColor 0.0 0.0 (/ 1.0 999.9) 0.0) :!class /Script/Engine.KismetMaterialLibrary)
  (Rendering|Material|SetVectorParameterValue "/Game/ShadowMap/MPC_LightParams.MPC_LightParams" "projectionW" (Utilities|Struct|MakeLinearColor 0.0 0.0 (/ -0.1 999.9) 1.0) :!class /Script/Engine.KismetMaterialLibrary))