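; Shadow-mapping light actor that uses an orthographic SceneCaptureComponent2D as the light's viewpoint, publishing its transform to the MPC_LightParams material parameter collection.
; The construction script writes the capture's position and a hand-built world-to-light view matrix from its axes and negated position dot products.
; It also writes projection rows derived from OrthoWidth and a hardcoded depth range.
; The event graph is empty, so values update only when construction reruns.
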(event EventBeginPlay)

(event Collision|EventActorBeginOverlap
  (params (OtherActor :type Actor%20Object%20Reference)))

(event EventTick
  (params (DeltaSeconds :type Float%20%28single-precision%29)))

(fn ConstructionScript
  (bind _scenecapturecomponent2d (Variables|Default|GetSceneCaptureComponent2D))
  (bind _scenecapturecomponent2d_2 (Variables|Default|GetSceneCaptureComponent2D))
  (bind _returnvalue (Math|Vector|GetRightVector _scenecapturecomponent2d))
  (bind _returnvalue_2 (Math|Vector|GetUpVector _scenecapturecomponent2d))
  (bind _returnvalue_3 (Math|Vector|GetForwardVector _scenecapturecomponent2d))
  (bind _returnvalue_4 (Transformation|GetWorldLocation _scenecapturecomponent2d))
  (bind _orthowidth (Variables|/Script/Engine.SceneCaptureComponent2D|GetOrthoWidth _scenecapturecomponent2d_2))
  (bind (_x _y _z) (Math|Vector|BreakVector _returnvalue_3))
  (bind (_x_2 _y_2 _z_2) (Math|Vector|BreakVector _returnvalue))
  (bind (_x_3 _y_3 _z_3) (Math|Vector|BreakVector _returnvalue_2))
  (Rendering|Material|SetVectorParameterValue "/Game/ShadowMap/MPC_LightParams.MPC_LightParams" "lightPos" (Math|Conversions|ToLinearColor(Vector) (Transformation|GetWorldLocation _scenecapturecomponent2d)) :!class /Script/Engine.KismetMaterialLibrary)
  (Rendering|Material|SetVectorParameterValue "/Game/ShadowMap/MPC_LightParams.MPC_LightParams" "lightMatrixX" (Utilities|Struct|MakeLinearColor _x_2 _x_3 _x 0.0) :!class /Script/Engine.KismetMaterialLibrary)
  (Rendering|Material|SetVectorParameterValue "/Game/ShadowMap/MPC_LightParams.MPC_LightParams" "lightMatrixY" (Utilities|Struct|MakeLinearColor _y_2 _y_3 _y 0.0) :!class /Script/Engine.KismetMaterialLibrary)
  (Rendering|Material|SetVectorParameterValue "/Game/ShadowMap/MPC_LightParams.MPC_LightParams" "lightMatrixZ" (Utilities|Struct|MakeLinearColor _z_2 _z_3 _z 0.0) :!class /Script/Engine.KismetMaterialLibrary)
  (Rendering|Material|SetVectorParameterValue "/Game/ShadowMap/MPC_LightParams.MPC_LightParams" "lightMatrixW" (Math|Conversions|ToLinearColor(Vector) (Math|Vector|MakeVector (* (Math|Vector|DotProduct _returnvalue _returnvalue_4) -1.0) (* (Math|Vector|DotProduct _returnvalue_2 _returnvalue_4) -1.0) (* (Math|Vector|DotProduct _returnvalue_3 _returnvalue_4) -1.0))) :!class /Script/Engine.KismetMaterialLibrary)
  (Rendering|Material|SetVectorParameterValue "/Game/ShadowMap/MPC_LightParams.MPC_LightParams" "projectionX" (Utilities|Struct|MakeLinearColor (/ _orthowidth 2.0) 0.0 0.0 0.0) :!class /Script/Engine.KismetMaterialLibrary)
  (Rendering|Material|SetVectorParameterValue "/Game/ShadowMap/MPC_LightParams.MPC_LightParams" "projectionY" (Utilities|Struct|MakeLinearColor 0.0 (/ _orthowidth -2.0) 0.0 0.0) :!class /Script/Engine.KismetMaterialLibrary)
  (Rendering|Material|SetVectorParameterValue "/Game/ShadowMap/MPC_LightParams.MPC_LightParams" "projectionZ" (Utilities|Struct|MakeLinearColor 0.0 0.0 (/ 1.0 1e+03) 0.0) :!class /Script/Engine.KismetMaterialLibrary)
  (Rendering|Material|SetVectorParameterValue "/Game/ShadowMap/MPC_LightParams.MPC_LightParams" "projectionW" (Utilities|Struct|MakeLinearColor 0.0 0.0 (/ -0.1 1e+03) 0.0) :!class /Script/Engine.KismetMaterialLibrary))